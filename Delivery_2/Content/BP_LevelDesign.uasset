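; BP_LevelDesign is a timed enemy spawner that keeps adding BP_Enemy actors to the level at random spawn points.
; On BeginPlay it caches every actor carrying SpawnerTag as a spawn point.
; Tick feeds an accumulating timer, and each time it reaches SpawnTime, Spawn resets it, creates an enemy at a random point's location and calls its OnSpawn.
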(event `self.ReceiveBeginPlay`
  (bind _outactors (`GameplayStatics.GetAllActorsWithTag` (`self.spawnerTag`)))
  (set `self.spawners` _outactors))

(event `self.ReceiveTick`
  (params (DeltaSeconds :type "Float (single-precision)"))
  (`self.UpdateTimers` DeltaSeconds))

(fn `Spawn`
  (set `self.spawnTimer` 0.0)
  (bind _returnvalue (`|SpawnActorFromClass` "/Game/LevelDesign_Tomás/Enemy/BP_Enemy.BP_Enemy_C" (`KismetMathLibrary.Conv_VectorToTransform` (`self.K2_GetActorLocation` (`KismetArrayLibrary.Array_Random` (`self.spawners`)))) "Undefined" "OverrideRootScale" null null))
  (`/Game/LevelDesign_Tomás/Enemy/BP_Enemy.OnSpawn` _returnvalue))

(fn `UpdateTimers`
  (params (dt :type "Float (double-precision)"))
  (bind _output_get (set `self.spawnTimer` (+ dt (`self.spawnTimer`))))
  (if (>= _output_get (`self.spawnTime`))
    (`self.Spawn`)))

(fn `UserConstructionScript`)